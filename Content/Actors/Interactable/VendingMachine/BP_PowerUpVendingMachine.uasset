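; BP_PowerUpVendingMachine is an interactable vending machine that grants a powerup to the player.
; On interaction, it constructs an object from PowerupClass, applies it to player 0's pawn and sets a Done flag.
; When Once is set and Done is true, it skips the parent's StartInteract and EnableInteraction, making the machine single-use.
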(event EventBeginPlay
  (|CallParentFunction) ; This node is disabled and will not be called.\nDrag off pins to build functionality.
)

(event Collision|EventActorBeginOverlap
  (params (OtherActor :type Actor%20Object%20Reference)))

(event EventTick
  (params (DeltaSeconds :type Float%20%28single-precision%29))
  (|CallParentFunction DeltaSeconds) ; This node is disabled and will not be called.\nDrag off pins to build functionality.
)

(event EventStartInteract
  (if (not (and (Variables|Default|GetOnce) (Variables|Default|GetDone)))
    (|CallParentFunction)))

(event EventEnableInteraction
  (if (not (and (Variables|Default|GetOnce) (Variables|Default|GetDone)))
    (|CallParentFunction)))

(fn ConstructionScript
  (|CallParentFunction))

(fn OnInteracted
  (|CallParentFunction)
  (bind _returnvalue (Game|ConstructObjectfromClass (Variables|Default|GetPowerupClass)))
  (Default|ApplyPowerup _returnvalue (Game|Player|GetPlayerPawn 0))
  (Variables|Default|SetDone true))