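; Base melee enemy that chases the player and attacks up close, with mesh, animations and capsule size from a data asset and a random audio cue.
; Tick switches between AI MoveTo at random walk/run speed and timed sphere-trace attacks, playing animations directly on the mesh.
; Incoming hits spawn blood, deal fixed heavy damage high on the body, trigger a one-time low-health stagger, then death and delayed destruction.
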(event Custom|Walk/Run%20Towards%20Player
  (bind _dataasset (Variables|Default|GetDataAsset))
  (Variables|Default|SetAttackStarted false)
  (Variables|Default|SetWalkStarted true)
  (Variables|/Script/Engine.CharacterMovementComponent|SetMaxWalkSpeed (Variables|Character|GetCharacterMovement) (Math|Random|RandomFloatinRange 2.5e+02 4.5e+02))
  (Components|Animation|PlayAnimation (Variables|Character|GetMesh) (select (Math|Float|InRange(Float) (Variables|/Script/Engine.CharacterMovementComponent|GetMaxWalkSpeed (Variables|Character|GetCharacterMovement)) 2.5e+02 325.0) (Variables|/Game/AI/Data/EnemyDataAssetClass.EnemyDataAssetClass_C|GetWalkAnim _dataasset) (Variables|/Game/AI/Data/EnemyDataAssetClass.EnemyDataAssetClass_C|GetRunAnim _dataasset)) true)
  (AI|AIMoveTo self "0, 0, 0" (Game|Player|GetPlayerPawn 0) 1.5e+02 false
    (:OnSuccess
      _)
    (:OnFail
      _))
  (Variables|Default|SetWalkStarted false))

(event Custom|Attack
  (bind _returnvalue (Transformation|GetActorLocation))
  (Variables|Default|SetAttackStarted true)
  (Components|Animation|PlayAnimation (Variables|Character|GetMesh) (Variables|/Game/AI/Data/EnemyDataAssetClass.EnemyDataAssetClass_C|GetAttackAnim (Variables|Default|GetDataAsset)) true)
  (bind _outhit (Class|KismetSystemLibrary|SphereTraceSinglebyProfile _returnvalue (+ _returnvalue (* (Transformation|GetActorForwardVector) 2.5e+02)) 75.0 "Pawn" false 0 "None" true))
  (Game|Damage|ApplyDamage (.hitactor _outhit) (Variables|Default|GetBase%20Damage) 0 0)
  (Utilities|FlowControl|Delay (Variables|Default|GetDurationBetweenAttacks))
  (Variables|Default|SetAttackStarted false))

(event Custom|GetHit
  (bind _dataasset (Variables|Default|GetDataAsset))
  (bind _gethitanim (Variables|/Game/AI/Data/EnemyDataAssetClass.EnemyDataAssetClass_C|GetGetHitAnim _dataasset))
  (if (not (Variables|Default|GetGetHitPlayed))
    (Variables|Default|SetPlayingHit true)
    (Variables|Default|SetGetHitPlayed true)
    (AI|Navigation|StopMovement (AI|GetAIController self))
    (Components|Animation|PlayAnimation (Variables|Character|GetMesh) _gethitanim false)
    (Utilities|FlowControl|Delay (Animation|GetPlayLength _gethitanim))
    (Variables|Default|SetPlayingHit false)))

(event Custom|Die
  (bind _capsulecomponent (Variables|Collision|GetCapsuleComponent))
  (Audio|Components|Audio|Stop (Variables|Default|GetAudio))
  (Default|CallOnDead)
  (Variables|Default|SetDead true)
  (Components|Animation|PlayAnimation (Variables|Character|GetMesh) (Variables|/Game/AI/Data/EnemyDataAssetClass.EnemyDataAssetClass_C|GetDeathAnim (Variables|Default|GetDataAsset)) false)
  (Collision|SetCollisionObjectType _capsulecomponent "ECC_Visibility")
  (Collision|SetCollisionResponsetoAllChannels _capsulecomponent "ECR_Ignore")
  (Collision|SetCollisionResponsetoChannel (Variables|Collision|GetCapsuleComponent) "ECC_WorldStatic" "ECR_Block")
  (AI|Navigation|StopMovement (AI|GetAIController self))
  (Utilities|FlowControl|Delay 2.0)
  (Actor|DestroyActor))

(event EventTick
  (params (DeltaSeconds :type Float%20%28single-precision%29))
  (if (not (Variables|Default|GetDead))
    (if (Math|Float|InRange(Float) (Math|Vector|Distance2D(Vector) (Transformation|GetActorLocation) (Transformation|GetActorLocation (Game|Player|GetPlayerPawn 0))) 0.0 2.5e+02)
      (if (not (Variables|Default|GetAttackStarted))
        (CallFunction|Attack))
      (elif (not (Variables|Default|GetPlayingHit))
        (if (not (Variables|Default|GetWalkStarted))
          (CallFunction|Walk/RunTowardsPlayer))))))

(event EventApplyDamage
  (params (Hit%20Result :type Hit%20Result%20Structure) (Damage :type Float%20%28double-precision%29))
  (bind _location (Collision|BreakHitResult Hit%20Result))
  (Niagara|SpawnSystematLocation "/Game/RealisticBlood/Burst/Niagara/NS_BloodBurst_Low.NS_BloodBurst_Low" _location)
  (if (not (Variables|Default|GetDead))
    (bind _output_get (Variables|Default|SetHealth (- (Variables|Default|GetHealth) (Math|Float|SelectFloat 1e+02 Damage (< (- (.z (Transformation|GetActorLocation)) (.Z (Math|Vector|BreakVector _location))) -2e+01)))))
    (if (<= _output_get 25.0)
      (CallFunction|GetHit)
      (if (<= (Variables|Default|GetHealth) 0.0)
        (CallFunction|Die)))))

(event EventBeginPlay
  (AI|SetFocus (AI|GetAIController self) (Game|Player|GetPlayerPawn 0))
  (CallFunction|Walk/RunTowardsPlayer))

(fn ConstructionScript
  (Components|SkeletalMesh|SetSkeletalMeshAsset (Variables|Character|GetMesh) (Variables|/Game/AI/Data/EnemyDataAssetClass.EnemyDataAssetClass_C|GetCharacterMesh (Variables|Default|GetDataAsset)))
  (Components|Capsule|SetCapsuleRadius (Variables|Collision|GetCapsuleComponent) (Variables|/Game/AI/Data/EnemyDataAssetClass.EnemyDataAssetClass_C|GetCapsuleRadius (Variables|Default|GetDataAsset)) true)
  (Components|Capsule|SetCapsuleHalfHeight (Variables|Collision|GetCapsuleComponent) (Variables|/Game/AI/Data/EnemyDataAssetClass.EnemyDataAssetClass_C|GetCapsuleHeight (Variables|Default|GetDataAsset)) true)
  (Transformation|AttachComponentToComponent (Variables|Default|GetCapsule) (Variables|Character|GetMesh) "Hips" "KeepRelative" "KeepRelative" "KeepRelative" true)
  (Audio|Components|Audio|SetSound (Variables|Default|GetAudio) (.OutItem (Utilities|Array|Random (Utilities|Array|MakeArray "/Game/Audio/Voices/Cue/Morley_Field_Sports_Complex_2-10_Cue.Morley_Field_Sports_Complex_2-10_Cue" "/Game/Audio/Voices/Cue/Morley_Field_Sports_Complex_2-11_Cue.Morley_Field_Sports_Complex_2-11_Cue" "/Game/Audio/Voices/Cue/Morley_Field_Sports_Complex_2-12_Cue.Morley_Field_Sports_Complex_2-12_Cue" "/Game/Audio/Voices/Cue/Morley_Field_Sports_Complex_2-13_Cue.Morley_Field_Sports_Complex_2-13_Cue" "/Game/Audio/Voices/Cue/Morley_Field_Sports_Complex_2-14_Cue.Morley_Field_Sports_Complex_2-14_Cue" "/Game/Audio/Voices/Cue/Morley_Field_Sports_Complex_2-15_Cue.Morley_Field_Sports_Complex_2-15_Cue" "/Game/Audio/Voices/Cue/Morley_Field_Sports_Complex_2-16_Cue.Morley_Field_Sports_Complex_2-16_Cue" "/Game/Audio/Voices/Cue/Morley_Field_Sports_Complex_2-17_Cue.Morley_Field_Sports_Complex_2-17_Cue" "/Game/Audio/Voices/Cue/Morley_Field_Sports_Complex_2-18_Cue.Morley_Field_Sports_Complex_2-18_Cue" "/Game/Audio/Voices/Cue/Morley_Field_Sports_Complex_2-19_Cue.Morley_Field_Sports_Complex_2-19_Cue" "/Game/Audio/Voices/Cue/Morley_Field_Sports_Complex_2-1_Cue.Morley_Field_Sports_Complex_2-1_Cue" "/Game/Audio/Voices/Cue/Morley_Field_Sports_Complex_2-20_Cue.Morley_Field_Sports_Complex_2-20_Cue" "/Game/Audio/Voices/Cue/Morley_Field_Sports_Complex_2-21_Cue.Morley_Field_Sports_Complex_2-21_Cue" "/Game/Audio/Voices/Cue/Morley_Field_Sports_Complex_2-22_Cue.Morley_Field_Sports_Complex_2-22_Cue" "/Game/Audio/Voices/Cue/Morley_Field_Sports_Complex_2-23_Cue.Morley_Field_Sports_Complex_2-23_Cue" "/Game/Audio/Voices/Cue/Morley_Field_Sports_Complex_2-24_Cue.Morley_Field_Sports_Complex_2-24_Cue" "/Game/Audio/Voices/Cue/Morley_Field_Sports_Complex_2-25_Cue.Morley_Field_Sports_Complex_2-25_Cue" "/Game/Audio/Voices/Cue/Morley_Field_Sports_Complex_2-26_Cue.Morley_Field_Sports_Complex_2-26_Cue" "/Game/Audio/Voices/Cue/Morley_Field_Sports_Complex_2-27_Cue.Morley_Field_Sports_Complex_2-27_Cue" "/Game/Audio/Voices/Cue/Morley_Field_Sports_Complex_2-28_Cue.Morley_Field_Sports_Complex_2-28_Cue" "/Game/Audio/Voices/Cue/Morley_Field_Sports_Complex_2-29_Cue.Morley_Field_Sports_Complex_2-29_Cue" "/Game/Audio/Voices/Cue/Morley_Field_Sports_Complex_2-2_Cue.Morley_Field_Sports_Complex_2-2_Cue" "/Game/Audio/Voices/Cue/Morley_Field_Sports_Complex_2-30_Cue.Morley_Field_Sports_Complex_2-30_Cue" "/Game/Audio/Voices/Cue/Morley_Field_Sports_Complex_2-31_Cue.Morley_Field_Sports_Complex_2-31_Cue" "/Game/Audio/Voices/Cue/Morley_Field_Sports_Complex_2-32_Cue.Morley_Field_Sports_Complex_2-32_Cue" "/Game/Audio/Voices/Cue/Morley_Field_Sports_Complex_2-33_Cue.Morley_Field_Sports_Complex_2-33_Cue" "/Game/Audio/Voices/Cue/Morley_Field_Sports_Complex_2-34_Cue.Morley_Field_Sports_Complex_2-34_Cue" "/Game/Audio/Voices/Cue/Morley_Field_Sports_Complex_2-35_Cue.Morley_Field_Sports_Complex_2-35_Cue" "/Game/Audio/Voices/Cue/Morley_Field_Sports_Complex_2-36_Cue.Morley_Field_Sports_Complex_2-36_Cue" "/Game/Audio/Voices/Cue/Morley_Field_Sports_Complex_2-37_Cue.Morley_Field_Sports_Complex_2-37_Cue" "/Game/Audio/Voices/Cue/Morley_Field_Sports_Complex_2-38_Cue.Morley_Field_Sports_Complex_2-38_Cue" "/Game/Audio/Voices/Cue/Morley_Field_Sports_Complex_2-3_Cue.Morley_Field_Sports_Complex_2-3_Cue" "/Game/Audio/Voices/Cue/Morley_Field_Sports_Complex_2-4_Cue.Morley_Field_Sports_Complex_2-4_Cue" "/Game/Audio/Voices/Cue/Morley_Field_Sports_Complex_2-5_Cue.Morley_Field_Sports_Complex_2-5_Cue" "/Game/Audio/Voices/Cue/Morley_Field_Sports_Complex_2-6__1__Cue.Morley_Field_Sports_Complex_2-6__1__Cue" "/Game/Audio/Voices/Cue/Morley_Field_Sports_Complex_2-6_Cue.Morley_Field_Sports_Complex_2-6_Cue" "/Game/Audio/Voices/Cue/Morley_Field_Sports_Complex_2-7_Cue.Morley_Field_Sports_Complex_2-7_Cue" "/Game/Audio/Voices/Cue/Morley_Field_Sports_Complex_2-8_Cue.Morley_Field_Sports_Complex_2-8_Cue" "/Game/Audio/Voices/Cue/Morley_Field_Sports_Complex_2-9_Cue.Morley_Field_Sports_Complex_2-9_Cue" "/Game/Audio/Voices/Cue/Morley_Field_Sports_Complex_2_Cue.Morley_Field_Sports_Complex_2_Cue")))))